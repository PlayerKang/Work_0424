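; Player-flown pawn that constantly moves forward and can fire rockets.
; BeginPlay adds the Enhanced Input mapping context through BP_ControllerF, and Tick feeds forward-vector input, scaled by delta time, into FloatingPawnMovement.
; Pitch and roll inputs rotate the actor in local space to steer, with no yaw input.
; The attack input spawns BP_Rocket at the Arrow component's world transform on each Triggered event.
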(event Input|EnhancedActionEvents|EnhancedInputActionIA_Pitch
  (params (ActionValue :type Float%20%28double-precision%29) (ElapsedSeconds :type Float%20%28double-precision%29) (TriggeredSeconds :type Float%20%28double-precision%29) (InputAction :type Input%20Action%20Object%20Reference :default "/Game/Input/IA_Pitch.IA_Pitch"))
  (:Triggered
    (Transformation|AddActorLocalRotation (Math|Rotator|MakeRotator 0.0 ActionValue 0.0) false false)))

(event Input|EnhancedActionEvents|EnhancedInputActionIA_Roll
  (params (ActionValue :type Float%20%28double-precision%29) (ElapsedSeconds :type Float%20%28double-precision%29) (TriggeredSeconds :type Float%20%28double-precision%29) (InputAction :type Input%20Action%20Object%20Reference :default "/Game/Input/IA_Roll.IA_Roll"))
  (:Triggered
    (Transformation|AddActorLocalRotation (Math|Rotator|MakeRotator ActionValue 0.0 0.0) false false)))

(event Input|EnhancedActionEvents|EnhancedInputActionIA_Attack
  (params (ActionValue :type Boolean) (ElapsedSeconds :type Float%20%28double-precision%29) (TriggeredSeconds :type Float%20%28double-precision%29) (InputAction :type Input%20Action%20Object%20Reference :default "/Game/Input/IA_Attack.IA_Attack"))
  (:Triggered
    (Game|SpawnActorfromClass "/Game/BluePrints/BP_Rocket.BP_Rocket_C" (Transformation|GetWorldTransform (Variables|Default|GetArrow)) "Undefined" 0 0)))

(event EventTick
  (params (DeltaSeconds :type Float%20%28single-precision%29))
  (Class|PawnMovementComponent|AddInputVector (Variables|Default|GetFloatingPawnMovement) (* (Transformation|GetActorForwardVector) (* DeltaSeconds 1e+02)) false))

(event EventBeginPlay
  (bind _asbp_controller_f (Utilities|Casting|CastToBP_ControllerF (Game|GetPlayerController 0)))
  (Input|AddMappingContext (PlayerController|LocalPlayerSubsystems|GetEnhancedInputLocalPlayerSubsystem _asbp_controller_f) "/Game/Input/IPC_Default.IPC_Default" 0 "(bIgnoreAllPressedKeysUntilRelease=True,bForceImmediately=False)"))

(fn ConstructionScript)